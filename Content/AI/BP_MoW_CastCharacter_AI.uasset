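; AI-controlled character that joins a random team, respawns at start and heads for capturable objectives its team does not own.
; After a short delay it uses SimpleMoveToActor toward a random such objective.
; A Tick timer periodically compares locations and, if it has not moved, redirects it to the nearest such objective.
; Capsule overlap with an opposing-team character triggers a melee attack; the projectile attack is unwired.
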(event OnComponentBeginOverlap(CapsuleComponent)
  (params (OtherActor :type Actor%20Object%20Reference) (OtherComp :type Primitive%20Component%20Object%20Reference) (OtherBodyIndex :type Integer) (bFromSweep :type Boolean) (SweepResult :type Hit%20Result%20Structure%20%28by%20ref%29))
  (bind _asbp_mo_w_base_character (Utilities|Casting|CastToBP_MoW_BaseCharacter OtherActor)
    (:then
      (if (!= (Variables|/Game/FirstPersonBP/Blueprints/Characters/BP_MoW_BaseCharacter.BP_MoW_BaseCharacter_C|GetPlayerTeam _asbp_mo_w_base_character) (Variables|Default|GetPlayerTeam))
        (CallFunction|MeleeAttack)))
    (:CastFailed
      (Utilities|Casting|CastToBP_DestructibleObject OtherActor))))

(event EventBeginPlay
  (CallFunction|ChangetoRandomTeam)
  (CallFunction|Respawn)
  (Utilities|FlowControl|Delay 5.0)
  (CallFunction|MovetoRandomObjective))

(event EventTick
  (params (DeltaSeconds :type Float%20%28single-precision%29))
  ;[1 1 1] Check if stuck / or have not moved for 5s
  (Variables|Default|SetStuckCheckTimer (+ (Variables|Default|GetStuckCheckTimer) DeltaSeconds))
  (if (> (Variables|Default|GetStuckCheckTimer) 5.0)
    (CallFunction|CheckifStuck)
    (Variables|Default|SetStuckCheckTimer 0.0)))

(fn ConstructionScript
  (|CallParentFunction))

(fn MovetoRandomObjective
  (bind _attackableobjectives (Variables|Default|GetAttackableObjectives))
  (Utilities|Array|Clear (Variables|Default|GetAttackableObjectives))
  (bind _outactors (Actor|GetAllActorsOfClass "/Game/FirstPersonBP/Blueprints/Objectives/CapturableObjective.CapturableObjective_C"))
  (for _array_element _outactors
    (if (!= (Variables|/Game/FirstPersonBP/Blueprints/Objectives/CapturableObjective.CapturableObjective_C|GetOwningTeam _array_element) (Variables|Default|GetPlayerTeam self))
      (bind _returnvalue (Utilities|Array|Add (Variables|Default|GetAttackableObjectives) _array_element))
      (Development|PrintText (Utilities|Text|ToText(Integer) _returnvalue) true true "(R=0.000000,G=0.660000,B=1.000000,A=1.000000)" 5.0)))
  (AI|Navigation|SimpleMovetoActor (Pawn|GetController self) (Utilities|Array|Get(acopy) _attackableobjectives (Math|Random|RandomIntegerinRange 0 (Utilities|Array|LastIndex _attackableobjectives)))))

(fn CheckifStuck
  (if (Math|Vector|Equal(Vector) (Variables|Default|GetStuckLocation) (Transformation|GetActorLocation) 0.0001)
    (CallFunction|MovetoNearestObjective)
    (else
      (Variables|Default|SetStuckLocation (Transformation|GetActorLocation)))))

(fn MovetoNearestObjective
  (bind _self self)
  (bind _attackableobjectives (Variables|Default|GetAttackableObjectives))
  ;[1 1 1] Clear current objective knowledge
  (Variables|Default|SetcurrentTargetObjective 0)
  (Utilities|Array|Clear (Variables|Default|GetAttackableObjectives))
  ;[1 1 1] Create list of attackable objectives
  (bind _outactors (Actor|GetAllActorsOfClass "/Game/FirstPersonBP/Blueprints/Objectives/CapturableObjective.CapturableObjective_C"))
  (for _array_element _outactors
    (if (!= (Variables|/Game/FirstPersonBP/Blueprints/Objectives/CapturableObjective.CapturableObjective_C|GetOwningTeam _array_element) (Variables|Default|GetPlayerTeam self))
      (Utilities|Array|Add (Variables|Default|GetAttackableObjectives) _array_element)))
  ;[1 1 1] Initialise current target before iteration
  (Variables|Default|SetcurrentTargetObjective (Utilities|Array|Get(acopy) _attackableobjectives))
  (for _array_element_2 _attackableobjectives
    ;[1 1 1] Find the closest objective that is owned by an enemy
    (if (and (< (Transformation|GetDistanceTo _array_element_2 _self) (Transformation|GetDistanceTo (Variables|Default|GetcurrentTargetObjective) _self)) (!= (Variables|/Game/FirstPersonBP/Blueprints/Objectives/CapturableObjective.CapturableObjective_C|GetOwningTeam (Variables|Default|GetcurrentTargetObjective)) (Variables|Default|GetPlayerTeam self)))
      (Variables|Default|SetcurrentTargetObjective _array_element_2)))
  ;[1 1 1] Move to current target
  (AI|Navigation|SimpleMovetoActor (Pawn|GetController self) (Variables|Default|GetcurrentTargetObjective)))